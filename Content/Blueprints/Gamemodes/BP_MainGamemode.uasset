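; Main game mode for a local multiplayer cat-versus-mice game, handling player spawning, shared UI and game over.
; BeginPlay gathers BP_Spawn points, creates GameInstance's active players, and possesses each with a cat (player 0) or mouse at random matching spawns.
; It adds a fullscreen stress bar; per-role split-screen widgets are unwired stubs.
; AdjustStressMeter triggers a cat-loss GameOver screen at maximum stress, while Tick debug-prints controller names.
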(event Custom|StartGame
  (Utilities|FlowControl|Delay 0.0)
  (CallFunction|SpawnAllCharacters)
  (CallFunction|CreatePlayerUI))

(event EventTick
  (params (DeltaSeconds :type Float%20%28single-precision%29))
  (bind _outactors (Actor|GetAllActorsOfClass "/Game/Blueprints/Controllers/BP_PlayerController.BP_PlayerController_C"))
  (for _array_element _outactors
    (Development|PrintString (Utilities|GetDisplayName _array_element) true true "(R=0.000000,G=0.660000,B=1.000000,A=1.000000)" (Utilities|Time|GetWorldDeltaSeconds))))

(event EventBeginPlay
  (bind _outactors (Actor|GetAllActorsOfClass "/Game/Blueprints/GenericActors/BP_Spawn.BP_Spawn_C"))
  (Variables|Default|SetAllSpawns _outactors)
  (CallFunction|StartGame))

(fn ConstructionScript)

(fn CreatePlayerUI
  ;[1 1 1] Loop through all players
  (bind _asbp_game_instance (Utilities|Casting|CastToBP_GameInstance (Game|GetGameInstance)))
  (bind _playeramount (Default|GetPlayerNumbers _asbp_game_instance))
  (for _array_element _playeramount
    (bind _asbp_player_controller (Utilities|Casting|CastToBP_PlayerController (Game|GetPlayerController _array_element)))
    (if (Utilities|Enum|Equal(Enum) (Variables|/Game/Blueprints/Controllers/BP_PlayerController.BP_PlayerController_C|GetCharacterType _asbp_player_controller) "NewEnumerator0")
      _))
  ;[1 1 1] Add fullscreen widgets here
  (bind _returnvalue (UserInterface|CreateWidget "/Game/Blueprints/UI/StressBarUI.StressBarUI_C" (Game|GetPlayerController 0)))
  (UserInterface|Viewport|AddtoViewport _returnvalue (.fullscreengame (Variables|UIRelated|GetUIZOrderStruct))))

(fn AdjustStressMeter
  (params (Adjust%20Amount :type Float%20%28single-precision%29))
  ;[1 1 1] Add stress meter value
  (if (>= (+ Adjust%20Amount (Variables|Default|GetStressMeterValue)) (Variables|Default|GetMaxStress))
    (Variables|Default|SetStressMeterValue (Variables|Default|GetMaxStress))
    (CallFunction|GameOver false)
    (else
      (bind _output_get (Variables|Default|SetStressMeterValue 0.0))
      (Development|PrintString (Utilities|String|Append "Stress meter level: " (Utilities|String|ToString(Float) _output_get)) true true "(R=0.000000,G=1.000000,B=0.031264,A=1.000000)"))))

(fn GameOver
  (params (DidCatWin? :type Boolean))
  (bind _returnvalue (UserInterface|CreateWidget "/Game/Blueprints/UI/GameOverScreen.GameOverScreen_C" 0 DidCatWin?))
  (UserInterface|Viewport|AddtoViewport _returnvalue 0))

(fn SpawnCharacter
  (params (Controller :type BP%20Player%20Controller%20Object%20Reference))
  (bind _selectablespawns (LocalVariables|GetSelectableSpawns))
  (bind _returnvalue (Utilities|Array|LastIndex _selectablespawns))
  (bind _returnvalue_2 (Math|Random|RandomIntegerinRange 0 _returnvalue))
  (bind _output (Utilities|Array|Get(acopy) _selectablespawns _returnvalue_2))
  (bind _returnvalue_3 (Transformation|GetActorTransform _output))
  ;[1 1 1] What type of player are we
  (bind _output_get (LocalVariables|SetPlayerCon Controller))
  (Variables|/Game/Blueprints/Controllers/BP_PlayerController.BP_PlayerController_C|SetCharacterType (LocalVariables|GetPlayerCon) (select (== (Class|GameplayStatics|GetPlayerControllerID _output_get) (Variables|Default|GetCatPlayerID)) "NewEnumerator0" "NewEnumerator1"))
  ;[1 1 1] Destroy old pawn
  (Utilities|IsValid (Pawn|GetControlledPawn (LocalVariables|GetPlayerCon))
    (:Is%20Valid
      (Actor|DestroyActor (Pawn|GetControlledPawn (LocalVariables|GetPlayerCon))))
    (:Is%20Not%20Valid
      _))
  (for _array_element (Variables|Default|GetAllSpawns)
    ;[1 1 1] Checks if the player can spawn here
    (if (Utilities|Enum|Equal(Enum) (Variables|/Game/Blueprints/GenericActors/BP_Spawn.BP_Spawn_C|GetSpawnType _array_element) (Variables|/Game/Blueprints/Controllers/BP_PlayerController.BP_PlayerController_C|GetCharacterType (LocalVariables|GetPlayerCon)))
      (if (not (Variables|/Game/Blueprints/GenericActors/BP_Spawn.BP_Spawn_C|GetInUse _array_element))
        (Utilities|Array|Add (LocalVariables|GetSelectableSpawns) _array_element))))
  ;[1 1 1] Spawn new character and possess it
  (Variables|/Game/Blueprints/GenericActors/BP_Spawn.BP_Spawn_C|SetInUse _output true)
  (switch Utilities|FlowControl|Switch|SwitchonE_CharacterType (Variables|/Game/Blueprints/Controllers/BP_PlayerController.BP_PlayerController_C|GetCharacterType (LocalVariables|GetPlayerCon))
    (:NewEnumerator0
      (bind _returnvalue_4 (Game|SpawnActorfromClass "/Game/Blueprints/Characters/BP_Cat.BP_Cat_C" _returnvalue_3 "AdjustIfPossibleButAlwaysSpawn" (LocalVariables|GetPlayerCon) 0))
      (Variables|/Game/Blueprints/Characters/BP_Character.BP_Character_C|SetPlayerID _returnvalue_4 (Class|GameplayStatics|GetPlayerControllerID (LocalVariables|GetPlayerCon)))
      (Pawn|Possess (LocalVariables|GetPlayerCon) _returnvalue_4))
    (:NewEnumerator1
      (bind _returnvalue_5 (Game|SpawnActorfromClass "/Game/Blueprints/Characters/BP_Mouse.BP_Mouse_C" _returnvalue_3 "AdjustIfPossibleButAlwaysSpawn" (LocalVariables|GetPlayerCon) 0))
      (Variables|/Game/Blueprints/Characters/BP_Character.BP_Character_C|SetPlayerID _returnvalue_5 (Class|GameplayStatics|GetPlayerControllerID (LocalVariables|GetPlayerCon)))
      (Pawn|Possess (LocalVariables|GetPlayerCon) _returnvalue_5))))

(fn SpawnAllCharacters
  ;[1 1 1] Pick a cat player
  (bind _asbp_game_instance (Utilities|Casting|CastToBP_GameInstance (Game|GetGameInstance)))
  (bind _playeramount (Default|GetNumPlayers _asbp_game_instance))
  (Variables|Default|SetCatPlayerID 0)
  ;[1 1 1] Spawn the characters
  (bind _keys (Utilities|Map|Keys (Variables|/Game/Blueprints/GameInstance/BP_GameInstance.BP_GameInstance_C|GetPlayers _asbp_game_instance)))
  (for _array_element _keys
    (if (.Value (Utilities|Map|Find (Variables|/Game/Blueprints/GameInstance/BP_GameInstance.BP_GameInstance_C|GetPlayers _asbp_game_instance) _array_element))
      (Class|GameplayStatics|CreatePlayer _array_element)
      (bind _asbp_player_controller (Utilities|Casting|CastToBP_PlayerController (Game|GetPlayerController _array_element)))
      (CallFunction|SpawnCharacter _asbp_player_controller))))

(fn RemoveNonPlayers
  (bind _asbp_game_instance (Utilities|Casting|CastToBP_GameInstance (Game|GetGameInstance)))
  (bind _keys (Utilities|Map|Keys (Variables|/Game/Blueprints/GameInstance/BP_GameInstance.BP_GameInstance_C|GetPlayers _asbp_game_instance)))
  (for _array_element _keys
    (Development|PrintString (Utilities|GetDisplayName (Game|GetPlayerController _array_element)))
    (if (not (.Value (Utilities|Map|Find (Variables|/Game/Blueprints/GameInstance/BP_GameInstance.BP_GameInstance_C|GetPlayers _asbp_game_instance) _array_element)))
      (Class|GameplayStatics|RemovePlayer (Game|GetPlayerController _array_element) false))))