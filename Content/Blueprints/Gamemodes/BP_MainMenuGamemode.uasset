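; Main menu game mode that trims local multiplayer down to the first player.
; On BeginPlay it removes player controllers 1 through 3 and destroys their pawns.
; A SwitchToLevel function opens the M_Test level by name.
; An unconnected graph section that would create extra players from the game instance's Players map keys never runs.
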(event EventBeginPlay
  (Class|GameplayStatics|RemovePlayer (Game|GetPlayerController 1) true)
  (Class|GameplayStatics|RemovePlayer (Game|GetPlayerController 2) true)
  (Class|GameplayStatics|RemovePlayer (Game|GetPlayerController 3) true))

(fn ConstructionScript)

(fn SwitchtoLevel
  (Game|OpenLevel(byName) "M_Test"))