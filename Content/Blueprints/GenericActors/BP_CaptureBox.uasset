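; Capture box actor where a cat deposits the mouse player it carries.
; On overlap, it detaches the mouse, disables its input and pickup, shows a capture UI, and moves it onto the box.
; It ends the game through the game mode once the caught count equals player count minus one.
; Finishing an interaction re-enables overlapping mice without lowering that count, though CanInteract always returns false here.
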(event OnComponentBeginOverlap(DetectCatWithMouseBox)
  (params (OverlappedComponent :type Primitive%20Component%20Object%20Reference) (OtherActor :type Actor%20Object%20Reference) (OtherComp :type Primitive%20Component%20Object%20Reference) (OtherBodyIndex :type Integer) (bFromSweep :type Boolean) (SweepResult :type Hit%20Result%20Structure%20%28by%20ref%29))
  (bind _asbp_cat (Utilities|Casting|CastToBP_Cat OtherActor))
  (if (Variables|/Game/Blueprints/Characters/BP_Cat.BP_Cat_C|GetHasMouse _asbp_cat)
    (Variables|/Game/Blueprints/Characters/BP_Cat.BP_Cat_C|SetHasMouse _asbp_cat false)
    (CallFunction|MouseCaught (Variables|/Game/Blueprints/Characters/BP_Cat.BP_Cat_C|GetCaughtMouseRef _asbp_cat))
    (Transformation|SetWorldLocation (Variables|/Script/Engine.Character|GetCapsuleComponent (Variables|/Game/Blueprints/Characters/BP_Cat.BP_Cat_C|GetCaughtMouseRef _asbp_cat)) (Transformation|GetWorldLocation (Variables|Default|GetCube)) false false)))

(event EventOnFinishInteract
  (params (Characters :type Array%20of%20BP%20Character%20Object%20References))
  (CallFunction|MiceReleased))

(fn ConstructionScript)

(fn MouseCaught
  (params (Mouse%20caught :type BP%20Mouse%20Object%20Reference))
  (bind _capsulecomponent (Variables|/Script/Engine.Character|GetCapsuleComponent Mouse%20caught))
  (Math|Integer|IncrementInt (Variables|Default|GetMiceCaught)
    (:%20%20
      (bind _asbp_player_controller (Utilities|Casting|CastToBP_PlayerController (Pawn|GetController Mouse%20caught)))
      (bind _returnvalue (UserInterface|CreateWidget "/Game/Blueprints/UI/CaptureUI.CaptureUI_C" _asbp_player_controller))
      (UserInterface|Viewport|AddtoPlayerScreen _returnvalue)
      (Utilities|Casting|CastToBP_MainGamemode (Game|GetGameMode))
      ;[1 1 1] Disable input an detach while caught
      (Input|DisableInput Mouse%20caught _asbp_player_controller)
      (Transformation|DetachFromActor Mouse%20caught "KeepWorld" "KeepWorld" "KeepWorld")
      (Variables|/Game/Blueprints/Characters/BP_Mouse.BP_Mouse_C|SetCanBePickedUp Mouse%20caught false)
      (Collision|SetCollisionEnabled _capsulecomponent "QueryAndPhysics")
      (Rendering|SetVisibility _capsulecomponent true true)
      (bind _asbp_game_instance (Utilities|Casting|CastToBP_GameInstance (Game|GetGameInstance)))
      (bind _playeramount (Default|GetNumPlayers _asbp_game_instance))
      (if (== (- _playeramount 1) (Variables|Default|GetMiceCaught))
        (bind _asbp_main_gamemode (Utilities|Casting|CastToBP_MainGamemode (Game|GetGameMode)))
        (Default|GameOver _asbp_main_gamemode true)))))

(fn MiceReleased
  (for _array_element (Collision|GetOverlappingActors (Variables|Default|GetDetectCatWithMouseBox) "/Game/Blueprints/Characters/BP_Mouse.BP_Mouse_C" :!class /Script/Engine.PrimitiveComponent)
    (bind _asbp_mouse (Utilities|Casting|CastToBP_Mouse _array_element))
    (bind _asplayer_controller (Utilities|Casting|CastToPlayerController (Pawn|GetController _asbp_mouse)))
    (Input|EnableInput _asbp_mouse _asplayer_controller)
    (Variables|/Game/Blueprints/Characters/BP_Mouse.BP_Mouse_C|SetCanBePickedUp _asbp_mouse true)
    (Development|PrintString "MICE ARE RELEASED" true true "(R=1.000000,G=0.048649,B=0.000000,A=1.000000)" 4.0)))

(fn CanInteract
  (params (Interactee :type BP%20Character%20Object%20Reference))
  (return false))