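; BP_Cat is the cat character, which jumps with a montage, catches player-controlled mice and handles object interaction.
; Interact releases a held mouse, or grabs a pickable mouse in MouseCatchBox and then drops a carried object or calls Interact.
; Capture teleports the mouse below the world, disables its input, blends its camera to the cat and shows capture widgets, which release reverses.
; Older line-trace interaction and pickup logic remains but is unreachable.
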(event EventBeginPlay
  (|CallParentFunction) ; This node is disabled and will not be called.\nDrag off pins to build functionality.
)

(event Collision|EventActorBeginOverlap
  (params (OtherActor :type Actor%20Object%20Reference))
  (|CallParentFunction OtherActor) ; This node is disabled and will not be called.\nDrag off pins to build functionality.
)

(event EventTick
  (params (DeltaSeconds :type Float%20%28single-precision%29))
  (|CallParentFunction DeltaSeconds) ; This node is disabled and will not be called.\nDrag off pins to build functionality.
)

(event EventOnJumped
  (Character|Jump)
  (Animation|PlayAnimMontage "/Game/Art/Animations/Cat/Anim_JumpStart.Anim_JumpStart" 1.0 "None"))

(event Input|ActionEvents|InputActionInteract
  (params (Key :type Key%20Structure))
  (:Pressed
    (if (Variables|Default|GetHasMouse)
      (CallFunction|ReleaseMouse)
      (else
        (for _array_element (Collision|GetOverlappingActors (Variables|Default|GetMouseCatchBox) "/Game/Blueprints/Characters/BP_Mouse.BP_Mouse_C" :!class /Script/Engine.PrimitiveComponent)
          (bind _asbp_mouse (Utilities|Casting|CastToBP_Mouse _array_element))
          (bind _asbp_player_controller (Utilities|Casting|CastToBP_PlayerController (Pawn|GetController _asbp_mouse)))
          (if (not (Variables|Default|GetHasMouse))
            (if (Variables|/Game/Blueprints/Characters/BP_Mouse.BP_Mouse_C|GetCanBePickedUp _asbp_mouse)
              (Variables|Default|SetHasMouse true)
              (Variables|Default|SetCaughtMousePlayerControllerRef _asbp_player_controller)
              (Variables|Default|SetCaughtMouseRef _asbp_mouse)
              (CallFunction|MouseCaught _asbp_player_controller _asbp_mouse))))
        (if (Variables|Default|GetCarryingObject)
          (CallFunction|DropObject false)
          (else
            (CallFunction|Interact))))))
  (:Released
    (CallFunction|StopInteract)))

(fn ConstructionScript
  (|CallParentFunction))

(fn MouseCaught
  (params (PlayercontrollerCaughtRef :type BP%20Player%20Controller%20Object%20Reference) (MouseCaughtRef :type BP%20Mouse%20Object%20Reference))
  (Utilities|IsValid (Variables|/Game/Blueprints/Characters/BP_Mouse.BP_Mouse_C|GetCarriedMouse MouseCaughtRef)
    (:Is%20Valid
      (Default|YEETmouse MouseCaughtRef))
    (:Is%20Not%20Valid
      (Audio|PlaySoundatLocation "/Game/Audio/Mouse/Cue_Caught.Cue_Caught" (Transformation|GetActorLocation) "0, 0, 0" 1.0 1.0 0.0 0 0 0)))
  (Game|Player|SetViewTargetwithBlend PlayercontrollerCaughtRef self 0.0 "VTBlend_EaseIn" 2.0 true)
  (Transformation|SetWorldLocation (Variables|/Script/Engine.Actor|GetRootComponent MouseCaughtRef) "0, 0,-500.000000" false true)
  (Input|DisableInput MouseCaughtRef PlayercontrollerCaughtRef)
  (bind _returnvalue (UserInterface|CreateWidget "/Game/Blueprints/UI/CaptureUI.CaptureUI_C" PlayercontrollerCaughtRef))
  (UserInterface|Viewport|AddtoPlayerScreen _returnvalue 5)
  (Variables|/Game/Blueprints/Characters/BP_Mouse.BP_Mouse_C|SetCapturedUIRef MouseCaughtRef _returnvalue)
  (Variables|/Game/Blueprints/Characters/BP_Mouse.BP_Mouse_C|SetCanBePickedUp MouseCaughtRef false)
  (bind _returnvalue_2 (UserInterface|CreateWidget "/Game/Blueprints/UI/CatCaptureUI.CatCaptureUI_C"))
  (UserInterface|Viewport|AddtoPlayerScreen _returnvalue_2)
  (Variables|Default|SetCatCaptureUiRef _returnvalue_2))

(fn ReleaseMouse
  (bind _caughtmouseplayercontrollerref (Variables|Default|GetCaughtMousePlayerControllerRef))
  (bind _caughtmouseref (Variables|Default|GetCaughtMouseRef))
  (Input|EnableInput _caughtmouseref _caughtmouseplayercontrollerref)
  (Variables|Default|SetHasMouse false)
  (Transformation|SetActorLocation _caughtmouseref (+ (Transformation|GetWorldLocation (Variables|Default|GetMouseCatchBox)) "0.000000, 0,50.000000") false false)
  (Game|Player|SetViewTargetwithBlend _caughtmouseplayercontrollerref _caughtmouseref 0.0 "VTBlend_EaseIn" 2.0 true)
  (Variables|/Game/Blueprints/Characters/BP_Mouse.BP_Mouse_C|SetCanBePickedUp _caughtmouseref true)
  (Widget|RemovefromParent (Variables|Default|GetCatCaptureUiRef)))