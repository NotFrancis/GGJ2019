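; BP_Bookcase is a furniture object that can tip over and adjusts the game mode's stress meter when it finishes falling.
; A second mesh previews the tipped pose in the construction script, then hides at BeginPlay, which registers the bookcase with its BP_BookcaseTipping child actor.
; Tip runs a timeline lerping the mesh's relative transform from its start to TipTransform, re-read at BeginPlay from the preview's world transform, and debug-prints it.
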(event Custom|Tip
  (bind _tiptransform (Variables|Default|GetTipTransform))
  (bind _newtrack_0 (Timeline|Timeline_0 PlayFromStart)
    (:Update
      (Transformation|SetRelativeTransform (Variables|Default|GetStaticMesh) (Math|Transform|Lerp(Transform) (Variables|Default|GetStartTransform) _tiptransform _newtrack_0) false false)
      (Development|PrintString (Utilities|String|ToString(Transform) _tiptransform) true true "(R=0.000000,G=0.660000,B=1.000000,A=1.000000)" (Utilities|Time|GetWorldDeltaSeconds)))
    (:Finished
      (bind _asbp_main_gamemode (Utilities|Casting|CastToBP_MainGamemode (Game|GetGameMode)))
      (Default|AdjustStressMeter _asbp_main_gamemode (Variables|Default|GetYeetStress)))))

(event EventBeginPlay
  (|CallParentFunction)
  (Variables|Default|SetStartTransform (Transformation|GetRelativeTransform (Variables|Default|GetStaticMesh)))
  (Variables|Default|SetTipTransform (Transformation|GetWorldTransform (Variables|Default|GetStaticMesh1)))
  (Rendering|SetVisibility (Variables|Default|GetStaticMesh1) false false)
  (bind _asbp_bookcase_tipping (Utilities|Casting|CastToBP_BookcaseTipping (Variables|/Script/Engine.ChildActorComponent|GetChildActor (Variables|Default|GetChildActor))))
  (Variables|/Game/Blueprints/Objects/Furniture/BP_BookcaseTipping.BP_BookcaseTipping_C|SetBookcase _asbp_bookcase_tipping self))

(event Collision|EventActorBeginOverlap
  (params (OtherActor :type Actor%20Object%20Reference))
  (|CallParentFunction OtherActor) ; This node is disabled and will not be called.\nDrag off pins to build functionality.
)

(event EventTick
  (params (DeltaSeconds :type Float%20%28single-precision%29))
  (|CallParentFunction DeltaSeconds) ; This node is disabled and will not be called.\nDrag off pins to build functionality.
)

(fn ConstructionScript
  (|CallParentFunction)
  (Transformation|SetRelativeTransform (Variables|Default|GetStaticMesh1) (Variables|Default|GetTipTransform) false false))