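; BP_DirtyItem is an object that spreads dirt to whatever it hits.
; On hit, it sends a dirty message to actors implementing BPI_Cleanable.
; Otherwise, if the hit static mesh actor uses a custom collision object type, it spawns a BP_PooStain at its own location, oriented along the impact normal.
; Debug strings print along each branch.
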(event EventBeginPlay
  (|CallParentFunction) ; This node is disabled and will not be called.\nDrag off pins to build functionality.
)

(event Collision|EventActorBeginOverlap
  (params (OtherActor :type Actor%20Object%20Reference))
  (|CallParentFunction OtherActor) ; This node is disabled and will not be called.\nDrag off pins to build functionality.
)

(event EventTick
  (params (DeltaSeconds :type Float%20%28single-precision%29))
  (|CallParentFunction DeltaSeconds) ; This node is disabled and will not be called.\nDrag off pins to build functionality.
)

(event EventOnHit
  (params (Actor :type Actor%20Object%20Reference) (HitResult :type Hit%20Result%20Structure))
  (bind _hitactor (Collision|BreakHitResult HitResult))
  (if (Utilities|DoesObjectImplementInterface Actor "/Game/Blueprints/Interfaces/BPI_Cleanable.BPI_Cleanable_C")
    (Class|BPICleanable|OnDirty(Message) Actor)
    (Development|PrintString "Object")
    (else
      (Development|PrintString (Utilities|GetDisplayName _hitactor))
      (bind _asstatic_mesh_actor (Utilities|Casting|CastToStaticMeshActor _hitactor))
      (Development|PrintString "bier")
      (if (Utilities|Enum|Equal(Enum) (Collision|GetCollisionObjectType (Variables|/Script/Engine.StaticMeshActor|GetStaticMeshComponent _asstatic_mesh_actor)) "ECC_GameTraceChannel1")
        (CallFunction|CreateDirtStain HitResult)
        (Development|PrintString "Stain")))))

(fn ConstructionScript
  (|CallParentFunction))

(fn CreateDirtStain
  (params (Hit :type Hit%20Result%20Structure))
  (Game|SpawnActorfromClass "/Game/Blueprints/Objects/BP_PooStain.BP_PooStain_C" (Math|Transform|MakeTransform (Transformation|GetActorLocation) (Math|Rotator|MakeRotationfromAxes (.impactnormal Hit) "0, 0, 0" "0, 0, 0") "2.000000,2.000000,2.000000") "Undefined" 0 0))