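; BP_InteractableObject is an interactable object with a timed interaction that can require several players at once.
; OnInteract adds the player to CurrentPlayers and, at PlayersNeeded, restarts InteractTimeline, rate-scaled by TimeToInteract, to drive each player's progress bar.
; OnStopInteract removes the player and stops the timeline when the count is at or below PlayersNeeded.
; OnFinishInteract is empty and never called here.
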(event EventBeginPlay
  (|CallParentFunction) ; This node is disabled and will not be called.\nDrag off pins to build functionality.
)

(event Collision|EventActorBeginOverlap
  (params (OtherActor :type Actor%20Object%20Reference))
  (|CallParentFunction OtherActor) ; This node is disabled and will not be called.\nDrag off pins to build functionality.
)

(event EventTick
  (params (DeltaSeconds :type Float%20%28single-precision%29))
  (|CallParentFunction DeltaSeconds) ; This node is disabled and will not be called.\nDrag off pins to build functionality.
)

(event EventOnInteract
  (params (Interactee :type BP%20Character%20Object%20Reference))
  (Utilities|Array|Add (Variables|Default|GetCurrentPlayers) Interactee)
  (if (>= (Utilities|Array|Length (Variables|Default|GetCurrentPlayers)) (Variables|Default|GetPlayersNeeded))
    (Components|Timeline|SetPlayRate (Variables|Default|GetInteractTimeline) (/ 1.0 (Variables|Default|GetTimeToInteract)))
    (bind _percentagedone (Timeline|InteractTimeline PlayFromStart)
      (:Update
        (for _array_element (Variables|Default|GetCurrentPlayers)
          (Progress|SetPercent (Variables|/Game/Blueprints/UI/W_InteractingTimer.W_InteractingTimer_C|GetProgressBar_40 (Variables|/Game/Blueprints/Characters/BP_Character.BP_Character_C|GetInteractingUI _array_element)) _percentagedone))))))

(event EventOnStopInteract
  (params (Interactee :type BP%20Character%20Object%20Reference))
  (Utilities|Array|RemoveItem (Variables|Default|GetCurrentPlayers) Interactee)
  (if (<= (Utilities|Array|Length (Variables|Default|GetCurrentPlayers)) (Variables|Default|GetPlayersNeeded))
    (bind _percentagedone (Timeline|InteractTimeline Stop)
      (:Update
        (for _array_element (Variables|Default|GetCurrentPlayers)
          (Progress|SetPercent (Variables|/Game/Blueprints/UI/W_InteractingTimer.W_InteractingTimer_C|GetProgressBar_40 (Variables|/Game/Blueprints/Characters/BP_Character.BP_Character_C|GetInteractingUI _array_element)) _percentagedone))))))

(fn ConstructionScript
  (|CallParentFunction))

(fn OnFinishInteract
  (params (NewParam :type BP%20Character%20Object%20Reference)))