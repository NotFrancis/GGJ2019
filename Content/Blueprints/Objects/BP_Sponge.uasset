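; BP_Sponge is an interactable cleaning tool that holds a Cleanliness charge.
; When its Box overlaps an actor while charge remains, it sends that actor OnCleanMessage with itself as argument, after printing a debug string.
; UseCharge deducts a fixed cost per clean and Clean refills the charge, though neither is called here.
; CanInteract admits only player controllers of the first CharacterType.
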(event OnComponentBeginOverlap(Box)
  (params (OverlappedComponent :type Primitive%20Component%20Object%20Reference) (OtherActor :type Actor%20Object%20Reference) (OtherComp :type Primitive%20Component%20Object%20Reference) (OtherBodyIndex :type Integer) (bFromSweep :type Boolean) (SweepResult :type Hit%20Result%20Structure%20%28by%20ref%29))
  (Development|PrintString (Utilities|String|Append "Overlap with: " (Utilities|GetDisplayName OtherActor)) true true "(R=0.447818,G=1.000000,B=0.501094,A=1.000000)")
  (if (> (Variables|Default|GetCleanliness) 0)
    (Class|BPICleanable|OnClean(Message) OtherActor self)))

(event EventBeginPlay
  (|CallParentFunction) ; This node is disabled and will not be called.\nDrag off pins to build functionality.
)

(event Collision|EventActorBeginOverlap
  (params (OtherActor :type Actor%20Object%20Reference))
  (|CallParentFunction OtherActor))

(fn ConstructionScript
  (|CallParentFunction))

(fn CanInteract
  (params (Interactee :type BP%20Character%20Object%20Reference))
  (|CallParentFunction Interactee)
  (bind _asbp_player_controller (Utilities|Casting|CastToBP_PlayerController (Pawn|GetController Interactee)))
  (return (Utilities|Enum|Equal(Enum) (Variables|/Game/Blueprints/Controllers/BP_PlayerController.BP_PlayerController_C|GetCharacterType _asbp_player_controller) "NewEnumerator0")))

(fn UseCharge
  (Variables|Default|SetCleanliness (- (Variables|Default|GetCleanliness) (Variables|Default|GetCleanlinessLostPerClean))))

(fn Clean
  (Variables|Default|SetCleanliness 100))